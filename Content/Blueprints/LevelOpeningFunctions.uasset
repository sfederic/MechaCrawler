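; Function library for level openings that switches the player's Mecha between cinematic and playable states and provides camera fades.
; LoadLevelWithSequence hides the Mecha, locks movement, plays the given level sequence and removes the shooting widget.
; LoadLevelPlayerMoveAndFadeIn reverses the Mecha changes and fades the camera and audio from full alpha.
; CameraFadeIn and CameraFadeOut both start at full alpha, differing only in that FadeOut holds when finished.
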(fn `CameraFadeIn`
  (`PlayerCameraManager.StartCameraFade` :`self` (`GameplayStatics.GetPlayerCameraManager` null) :`FromAlpha` 1.0 :`Duration` 2.0 :`bShouldFadeAudio` true))

(fn `CameraFadeOut`
  (`PlayerCameraManager.StartCameraFade` :`self` (`GameplayStatics.GetPlayerCameraManager` null) :`FromAlpha` 1.0 :`Duration` 2.0 :`bShouldFadeAudio` true :`bHoldWhenFinished` true))

(fn `LoadLevelPlayerMoveAndFadeIn`
  (bind _asmecha (cast `Mecha` (`GameplayStatics.GetPlayerPawn` null))
    (:`then`
      (`Actor.SetActorHiddenInGame` _asmecha false)
      (set `Mecha.canMove` true _asmecha)
      (`PlayerCameraManager.StartCameraFade` :`self` (`GameplayStatics.GetPlayerCameraManager` null) :`FromAlpha` 1.0 :`Duration` 3.0 :`bShouldFadeAudio` true)
      (`UserWidget.AddToViewport` (`Mecha.shootingWidget` _asmecha) 0))
    (:`CastFailed`
      (`KismetSystemLibrary.PrintString` null "Cast failed"))))

(fn `LoadLevelWithSequence`
  (params (Shot :type "LevelSequence Object Reference"))
  (locals (LevelSequence :type "LevelSequence Object Reference"))
  (bind _asmecha (cast `Mecha` (`GameplayStatics.GetPlayerPawn` null))
    (:`then`
      (`Actor.SetActorHiddenInGame` _asmecha true)
      (set `Mecha.canMove` false _asmecha)
      (bind (_outactor _returnvalue) (`LevelSequencePlayer.CreateLevelSequencePlayer` (`local.__WorldContext`) Shot))
      (`MovieSceneSequencePlayer.Play` _returnvalue)
      (`Widget.RemoveFromParent` (`Mecha.shootingWidget` _asmecha)))
    (:`CastFailed`
      (`KismetSystemLibrary.PrintString` null "Cast Failed"))))