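; BP_AudioTrigger is a level trigger that plays a sound when a Mecha overlaps it.
; The overlap event plays the Sound variable at the location of the referenced SoundOrigin actor, so the audio source can sit apart from the trigger.
; If IsOneShot is set, it then hides itself, disables its tick and turns off Box collision instead of being destroyed.
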(event `self.ReceiveActorBeginOverlap`
  (params (OtherActor :type "Actor Object Reference"))
  (cast `Mecha` OtherActor)
  (`GameplayStatics.PlaySoundAtLocation` (`self.sound`) (`self.K2_GetActorLocation` (`self.soundOrigin`)) (struct) 1.0 1.0 0.0 null null null)
  (if (`self.bIsOneShot`)
    (`self.SetActorHiddenInGame` true)
    (`self.SetActorTickEnabled` false)
    (`PrimitiveComponent.SetCollisionEnabled` (`self.Box`) "NoCollision")))

(fn `UserConstructionScript`)