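; Dialogue box child that ends the opening level with a hard cut to the title, then loads SecondLevel.
; On overlap it runs the parent's overlap logic, starts a timer and disables movement on the player's Mecha.
; When the timer fires, it snaps the camera to black, clears all widgets and shows BP_TitleHardCut.
; A second timer then opens the next level.
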(event `self.ReceiveActorBeginOverlap`
  (params (OtherActor :type "Actor Object Reference"))
  (`parent.ReceiveActorBeginOverlap` OtherActor)
  (`KismetSystemLibrary.K2_SetTimerDelegate` (delegate `HardCutToTitle`) 25.0)
  (bind _asmecha (cast `Mecha` (`GameplayStatics.GetPlayerPawn` 0)))
  (set `Mecha.canMove` false _asmecha))

(event `HardCutToTitle`
  ;[1 1 1] Just to create a hard cut to the title at the end of the opening level
  (`PlayerCameraManager.StartCameraFade` :`self` (`GameplayStatics.GetPlayerCameraManager` 0) :`ToAlpha` 1.0 :`Duration` 0.01 :`bHoldWhenFinished` true)
  (`WidgetLayoutLibrary.RemoveAllWidgets`)
  (bind _returnvalue (`|CreateWidget` "/Game/Blueprints/Widgets/BP_TitleHardCut.BP_TitleHardCut_C"))
  (`UserWidget.AddToViewport` _returnvalue 0)
  (`KismetSystemLibrary.K2_SetTimerDelegate` (delegate `OpenSecondLevel`) 10.0))

(event `OpenSecondLevel`
  (`GameplayStatics.OpenLevel` "SecondLevel"))

(fn `UserConstructionScript`
  (`parent.UserConstructionScript`))